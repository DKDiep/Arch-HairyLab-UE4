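; BP_ViewerPawn is a viewer pawn with a spring arm that supports zoom and rotation input.
; BeginPlay sets the spring arm's starting transform, and the zoom axis changes its arm length scaled by ScrollSpeed.
; An IsRotating toggle gates rotation of the scene root, with both X and Y axis events sharing one path that adds AxisValue to pitch and yaw together.
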(event Custom|InputZoomAxis_Event
  (params (AxisValue :type Float%20%28single-precision%29))
  (bind _springarm (Variables|Default|GetSpringArm))
  ;[1 1 1] Navigation
  (Variables|/Script/Engine.SpringArmComponent|SetTargetArmLength _springarm (- (Variables|/Script/Engine.SpringArmComponent|GetTargetArmLength _springarm) (* (Variables|Default|GetScrollSpeed) AxisValue))))

(event Custom|InputRotateOff_Event
  ;[1 1 1] Navigation
  (Variables|Default|SetIsRotating false))

(event Custom|InputRotateX_Event
  (params (AxisValue :type Float%20%28single-precision%29))
  (bind _defaultsceneroot (Variables|Default|GetDefaultSceneRoot))
  (bind _returnvalue (Transformation|GetRelativeTransform _defaultsceneroot))
  ;[1 1 1] Navigation
  (if (Variables|Default|GetIsRotating)
    (Transformation|SetRelativeTransform _defaultsceneroot (Math|Transform|MakeTransform "0, 0, 0" (Math|Rotator|MakeRotator 0.0 (+ (.pitch (.rotation _returnvalue)) (stale Custom|InputRotateY_Event AxisValue)) (+ (.yaw (.rotation _returnvalue)) AxisValue)) "1,1,1") false false)))

(event Custom|InputRotateOn_Event
  ;[1 1 1] Navigation
  (Variables|Default|SetIsRotating true))

(event Custom|InputRotateY_Event
  (params (AxisValue :type Float%20%28single-precision%29))
  (bind _defaultsceneroot (Variables|Default|GetDefaultSceneRoot))
  (bind _returnvalue (Transformation|GetRelativeTransform _defaultsceneroot))
  ;[1 1 1] Navigation
  (if (Variables|Default|GetIsRotating)
    (Transformation|SetRelativeTransform _defaultsceneroot (Math|Transform|MakeTransform "0, 0, 0" (Math|Rotator|MakeRotator 0.0 (+ (.pitch (.rotation _returnvalue)) AxisValue) (+ (.yaw (.rotation _returnvalue)) (stale Custom|InputRotateX_Event AxisValue))) "1,1,1") false false)))

(event EventBeginPlay
  (Transformation|SetWorldTransform (Variables|Default|GetSpringArm) (Math|Transform|MakeTransform "0.000000,0.000000,250.000000" "-15.000000,-20.000000,0.000000" "1.000000,1,1") false false))

(event Collision|EventActorBeginOverlap
  (params (OtherActor :type Actor%20Object%20Reference)))

(event EventTick
  (params (DeltaSeconds :type Float%20%28single-precision%29)))

(fn ConstructionScript)