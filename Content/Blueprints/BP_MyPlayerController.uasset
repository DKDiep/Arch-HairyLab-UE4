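; Player controller for a hair-placement viewer that spawns hair locks on a head model and passes camera input to BP_ViewerPawn.
; Left click traces under the cursor, spawns BP_Hair on BP_Head aligned to the surface normal, and builds a procedural quad on it.
; While the button is held, mouse movement rotates the new lock.
; Mouse movement always feeds pawn rotation, while wheel zoom and right-button rotate toggling work only outside place mode.
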(event EventBeginPlay)

(event EventTick
  (params (DeltaSeconds :type Float%20%28single-precision%29)))

(event Input|MouseEvents|MouseWheelAxis
  (params (AxisValue :type Float%20%28single-precision%29))
  (if (not (Variables|Default|GetisPlaceMode))
    (bind _asbp_viewer_pawn (Utilities|Casting|CastToBP_ViewerPawn (Game|Player|GetPlayerPawn 0)))
    (Default|InputZoomAxisEvent _asbp_viewer_pawn AxisValue)))

(event Input|MouseEvents|MouseX
  (params (AxisValue :type Float%20%28single-precision%29))
  (bind _currenthair (Variables|Default|GetCurrentHair))
  (bind _asbp_viewer_pawn (Utilities|Casting|CastToBP_ViewerPawn (Game|Player|GetPlayerPawn 0)))
  (Default|InputRotateXEvent _asbp_viewer_pawn AxisValue)
  (if (Variables|Default|GetisPlaceMode)
    (Utilities|IsValid _currenthair
      (:Is%20Valid
        (Transformation|AddActorLocalRotation _currenthair (Math|Rotator|MakeRotator 0.0 (* (stale Input|MouseEvents|MouseY AxisValue) 1e+01) (* AxisValue 1e+01)) false false)))))

(event Input|MouseEvents|MouseY
  (params (AxisValue :type Float%20%28single-precision%29))
  (bind _currenthair (Variables|Default|GetCurrentHair))
  (bind _asbp_viewer_pawn (Utilities|Casting|CastToBP_ViewerPawn (Game|Player|GetPlayerPawn 0)))
  (Default|InputRotateYEvent _asbp_viewer_pawn AxisValue)
  (if (Variables|Default|GetisPlaceMode)
    (Utilities|IsValid _currenthair
      (:Is%20Valid
        (Transformation|AddActorLocalRotation _currenthair (Math|Rotator|MakeRotator 0.0 (* AxisValue 1e+01) (* (stale Input|MouseEvents|MouseX AxisValue) 1e+01)) false false)))))

(event Input|MouseEvents|LeftMouseButton
  (params (Key :type Key%20Structure :default "AnyKey"))
  (:Pressed
    (bind _outhair (CallFunction|SpawnHair))
    (bind _output_get (Variables|Default|SetCurrentHair _outhair))
    (CallFunction|CreateMesh _output_get)
    (Variables|Default|SetisPlaceMode true))
  (:Released
    (Variables|Default|SetisPlaceMode false)))

(event Input|MouseEvents|RightMouseButton
  (params (Key :type Key%20Structure :default "AnyKey"))
  (bind _isplacemode (Variables|Default|GetisPlaceMode))
  (:Pressed
    (if (not _isplacemode)
      (bind _asbp_viewer_pawn (Utilities|Casting|CastToBP_ViewerPawn (Game|Player|GetPlayerPawn 0)))
      (Default|InputRotateonEvent _asbp_viewer_pawn)))
  (:Released
    (if (not _isplacemode)
      (bind _asbp_viewer_pawn_2 (Utilities|Casting|CastToBP_ViewerPawn (Game|Player|GetPlayerPawn 0)))
      (Default|InputRotateOffEvent _asbp_viewer_pawn_2))))

(fn ConstructionScript)

(fn SpawnHair
  (bind _hitresult (Game|Player|GetHitResultUnderCursorbyChannel "TraceTypeQuery1" true))
  (Variables|Default|SetHitLocation (.location _hitresult))
  (Variables|Default|SetHitNormal (.impactnormal _hitresult))
  (if (Utilities|ClassIsChildOf (Utilities|GetClass (.hitactor _hitresult)) "/Game/Blueprints/BP_Head.BP_Head_C")
    (bind _returnvalue (Game|SpawnActorfromClass "/Game/Blueprints/BP_Hair.BP_Hair_C" (Math|Transform|MakeTransform (Variables|Default|GetHitLocation) (Math|Rotator|FindLookatRotation (Variables|Default|GetHitLocation) (+ (Variables|Default|GetHitLocation) (Variables|Default|GetHitNormal))) "1,1,1") "AlwaysSpawn" 0 0))
    (Utilities|Array|Add (Variables|Default|GetHairLocks) _returnvalue))
  (return _returnvalue))

(fn CreateMesh
  (params (InHair :type Actor%20Object%20Reference))
  (bind _returnvalue (Actor|GetComponentsByClass InHair "/Script/ProceduralMeshComponent.ProceduralMeshComponent"))
  (bind _item (Utilities|Array|Get(acopy) _returnvalue))
  (Utilities|IsValid InHair
    (:Is%20Valid
      (if (>= (Utilities|Array|Length _returnvalue) 1)
        (Class|ProceduralMeshComponent|CreateMeshSectionLinearColor _item 0 (Utilities|Array|MakeArray "0.000000,-30.000000,0.000000" "0.000000,30.000000,0.000000" "100.000000,30.000000,0.000000" "100.000000,-30.000000, 0") (Utilities|Array|MakeArray 0 1 2 2 3 0) 0 0 0 0 false)
        (Rendering|Material|SetMaterial _item 0 "/Game/Materials/M_Test.M_Test")))
    (:Is%20Not%20Valid
      _))
  (return))